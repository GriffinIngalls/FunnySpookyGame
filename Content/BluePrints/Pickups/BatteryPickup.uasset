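; BatteryPickup is a pickup actor that recharges the Battery value of BP_FirstPersonCharacter.
; On overlap it casts the other actor to that character and, unless Battery is already full, adds a fixed charge capped at the maximum.
; The pickup destroys itself once used, and stays in the world when the battery is full.
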(event Collision|EventActorBeginOverlap
  (params (OtherActor :type Actor%20Object%20Reference))
  (bind _asbp_first_person_character (Utilities|Casting|CastToBP_FirstPersonCharacter OtherActor))
  (if (not (== (Variables|/Game/FirstPerson/Blueprints/BP_FirstPersonCharacter.BP_FirstPersonCharacter_C|GetBattery _asbp_first_person_character) 1e+02))
    (Variables|/Game/FirstPerson/Blueprints/BP_FirstPersonCharacter.BP_FirstPersonCharacter_C|SetBattery _asbp_first_person_character (+ (Variables|/Game/FirstPerson/Blueprints/BP_FirstPersonCharacter.BP_FirstPersonCharacter_C|GetBattery _asbp_first_person_character) 15.0))
    (if (>= (Variables|/Game/FirstPerson/Blueprints/BP_FirstPersonCharacter.BP_FirstPersonCharacter_C|GetBattery _asbp_first_person_character) 1e+02)
      (Variables|/Game/FirstPerson/Blueprints/BP_FirstPersonCharacter.BP_FirstPersonCharacter_C|SetBattery _asbp_first_person_character 1e+02)
      (Actor|DestroyActor)
      (else
        (Actor|DestroyActor)))))

(fn ConstructionScript)