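; FlickeringLight is a lighting Blueprint that makes a spotlight flicker on a fixed, repeating pattern.
; On BeginPlay a looping chain of retriggerable delays sets the SpotLight intensity between off, half and full brightness.
; The sequence mixes brief blinks with multi-second holds and has no randomness, and the construction script is empty.
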(event EventBeginPlay
  (Utilities|FlowControl|RetriggerableDelay 1e+01 :!label _label)
  (Rendering|Components|Light|SetIntensity (Variables|Default|GetSpotLight) 0.0)
  (Utilities|FlowControl|RetriggerableDelay 0.2)
  (Rendering|Components|Light|SetIntensity (Variables|Default|GetSpotLight) 1e+03)
  (Utilities|FlowControl|RetriggerableDelay 0.2)
  (Rendering|Components|Light|SetIntensity (Variables|Default|GetSpotLight) 0.0)
  (Utilities|FlowControl|RetriggerableDelay 5.0)
  (Rendering|Components|Light|SetIntensity (Variables|Default|GetSpotLight) 5e+02)
  (Utilities|FlowControl|RetriggerableDelay 5.0)
  (Rendering|Components|Light|SetIntensity (Variables|Default|GetSpotLight) 1e+03)
  (Utilities|FlowControl|RetriggerableDelay 15.0)
  (Rendering|Components|Light|SetIntensity (Variables|Default|GetSpotLight) 0.0)
  (Utilities|FlowControl|RetriggerableDelay 5.0)
  (Rendering|Components|Light|SetIntensity (Variables|Default|GetSpotLight) 1e+03)
  (goto _label))

(fn ConstructionScript)