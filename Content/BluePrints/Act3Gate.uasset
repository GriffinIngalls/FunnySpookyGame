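; Act 3 gate actor that removes itself once the game instance records LevelCompleted equal to 2.
; Every Tick it casts the game instance to UniversalVariables and polls that value.
; When the value matches, it resets the shared pressed, swap and switch flags to false, then destroys itself.
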(event EventTick
  (params (DeltaSeconds :type Float%20%28single-precision%29))
  (bind _asuniversal_variables (Utilities|Casting|CastToUniversalVariables (Game|GetGameInstance)))
  (if (== (Variables|/Game/BluePrints/UniversalVariables.UniversalVariables_C|GetLevelCompleted _asuniversal_variables) 2)
    (Variables|/Game/BluePrints/UniversalVariables.UniversalVariables_C|SetPressed? _asuniversal_variables false)
    (Variables|/Game/BluePrints/UniversalVariables.UniversalVariables_C|SetSwapColor _asuniversal_variables false)
    (Variables|/Game/BluePrints/UniversalVariables.UniversalVariables_C|SetSwapSwitch _asuniversal_variables false)
    (Variables|/Game/BluePrints/UniversalVariables.UniversalVariables_C|SetSwitchColor _asuniversal_variables false)
    (Variables|/Game/BluePrints/UniversalVariables.UniversalVariables_C|SetSwitchOnOff _asuniversal_variables false)
    (Actor|DestroyActor)))

(fn ConstructionScript)