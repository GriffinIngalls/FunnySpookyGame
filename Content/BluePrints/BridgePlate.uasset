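; BridgePlate is a pressure plate that reports whether a bridge trigger is pressed.
; When an actor tagged Heavy begins overlapping its Box, it sets BridgePressed on the UniversalVariables Game Instance and turns the RectLight blue.
; Any end overlap clears the flag and turns the light red, without checking the tag or whether a Heavy actor remains.
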(event OnComponentBeginOverlap(Box)
  (params (OverlappedComponent :type Primitive%20Component%20Object%20Reference) (OtherActor :type Actor%20Object%20Reference) (OtherComp :type Primitive%20Component%20Object%20Reference) (OtherBodyIndex :type Integer) (bFromSweep :type Boolean) (SweepResult :type Hit%20Result%20Structure%20%28by%20ref%29))
  (if (Actor|ActorHasTag OtherActor "Heavy")
    (bind _asuniversal_variables (Utilities|Casting|CastToUniversalVariables (Game|GetGameInstance)))
    (Variables|/Game/BluePrints/UniversalVariables.UniversalVariables_C|SetBridgePressed? _asuniversal_variables true)
    (Rendering|Components|Light|SetLightColor (Variables|Default|GetRectLight) (Class|KismetMathLibrary|LinearColorBlue) true)))

(event OnComponentEndOverlap(Box)
  (params (OverlappedComponent :type Primitive%20Component%20Object%20Reference) (OtherActor :type Actor%20Object%20Reference) (OtherComp :type Primitive%20Component%20Object%20Reference) (OtherBodyIndex :type Integer))
  (bind _asuniversal_variables (Utilities|Casting|CastToUniversalVariables (Game|GetGameInstance)))
  (Variables|/Game/BluePrints/UniversalVariables.UniversalVariables_C|SetBridgePressed? _asuniversal_variables false)
  (Rendering|Components|Light|SetLightColor (Variables|Default|GetRectLight) (Class|KismetMathLibrary|LinearColorRed) true))

(fn ConstructionScript)