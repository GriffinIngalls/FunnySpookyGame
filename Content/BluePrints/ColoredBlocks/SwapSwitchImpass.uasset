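; SwapSwitchImpass is a colored-block switch that toggles the global swap state whenever something begins overlapping its Box.
; The overlap flips SwapSwitch and sets SwapColor to match, both stored on the UniversalVariables game instance, with no filter on the overlapping actor.
; Tick polls SwapColor every frame to show or hide the BlueSwitch component, so its look follows the shared state.
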(event OnComponentBeginOverlap(Box)
  (params (OverlappedComponent :type Primitive%20Component%20Object%20Reference) (OtherActor :type Actor%20Object%20Reference) (OtherComp :type Primitive%20Component%20Object%20Reference) (OtherBodyIndex :type Integer) (bFromSweep :type Boolean) (SweepResult :type Hit%20Result%20Structure%20%28by%20ref%29))
  (bind _asuniversal_variables (Utilities|Casting|CastToUniversalVariables (Game|GetGameInstance)))
  (if (Variables|/Game/BluePrints/UniversalVariables.UniversalVariables_C|GetSwapSwitch _asuniversal_variables)
    (Variables|/Game/BluePrints/UniversalVariables.UniversalVariables_C|SetSwapSwitch _asuniversal_variables false)
    (Variables|/Game/BluePrints/UniversalVariables.UniversalVariables_C|SetSwapColor _asuniversal_variables false)
    (else
      (Variables|/Game/BluePrints/UniversalVariables.UniversalVariables_C|SetSwapSwitch _asuniversal_variables true)
      (Variables|/Game/BluePrints/UniversalVariables.UniversalVariables_C|SetSwapColor _asuniversal_variables true))))

(event EventTick
  (params (DeltaSeconds :type Float%20%28single-precision%29))
  (bind _blueswitch (Variables|Default|GetBlueSwitch))
  (bind _asuniversal_variables (Utilities|Casting|CastToUniversalVariables (Game|GetGameInstance)))
  (if (Variables|/Game/BluePrints/UniversalVariables.UniversalVariables_C|GetSwapColor _asuniversal_variables)
    (Rendering|SetVisibility _blueswitch true false)
    (else
      (Rendering|SetVisibility _blueswitch false false))))

(fn ConstructionScript)