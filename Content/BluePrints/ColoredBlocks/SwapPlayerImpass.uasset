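; SwapPlayerImpass is a block that swaps between a player impass and an item impass component based on a global switch.
; Every Tick it casts the GameInstance to UniversalVariables and reads SwapSwitch.
; When the switch is on, ItemImpass is visible with query and physics collision while PlayerImpass is hidden without collision; when off, the roles reverse.
; The state is polled and reapplied each frame rather than event-driven.
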(event EventBeginPlay)

(event Collision|EventActorBeginOverlap
  (params (OtherActor :type Actor%20Object%20Reference)))

(event EventTick
  (params (DeltaSeconds :type Float%20%28single-precision%29))
  (bind _playerimpass (Variables|Default|GetPlayerImpass))
  (bind _itemimpass (Variables|Default|GetItemImpass))
  (bind _asuniversal_variables (Utilities|Casting|CastToUniversalVariables (Game|GetGameInstance)))
  (if (Variables|/Game/BluePrints/UniversalVariables.UniversalVariables_C|GetSwapSwitch _asuniversal_variables)
    (Rendering|SetVisibility _playerimpass false false)
    (Collision|SetCollisionEnabled _playerimpass "NoCollision")
    (Rendering|SetVisibility _itemimpass true false)
    (Collision|SetCollisionEnabled _itemimpass "QueryAndPhysics")
    (else
      (Rendering|SetVisibility _playerimpass true false)
      (Collision|SetCollisionEnabled _playerimpass "QueryAndPhysics")
      (Rendering|SetVisibility _itemimpass false false)
      (Collision|SetCollisionEnabled _itemimpass "NoCollision"))))

(fn ConstructionScript)